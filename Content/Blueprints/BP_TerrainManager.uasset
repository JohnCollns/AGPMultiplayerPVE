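; Terrain manager that spawns mirrored counterparts of terrain actors on the other side of world X = 0.
; SpawnObjects spawns the passed Terrain's class with negated X position and yaw, keeping the other transform values.
; Each copy is added to MirrorObjects, runs MirrorStates and is logged with a debug print.
; A disconnected BaseWall cast for copying the wall mesh never runs.
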(event `self.SpawnObjects`
  (params (Terrain :type "TerrainMover Object Reference"))
  (bind _returnvalue (`GameplayStatics.GetObjectClass` Terrain))
  (if (`KismetSystemLibrary.IsValidClass` _returnvalue)
    (bind _returnvalue_2 (`|SpawnActorFromClass` _returnvalue (`KismetMathLibrary.MakeTransform` (`KismetMathLibrary.MakeVector` (* (.x (`self.K2_GetActorLocation` Terrain)) -1.0) (.y (`self.K2_GetActorLocation` Terrain)) (.z (`self.K2_GetActorLocation` Terrain))) (`KismetMathLibrary.MakeRotator` (.roll (`self.K2_GetActorRotation` Terrain)) (.pitch (`self.K2_GetActorRotation` Terrain)) (* (.yaw (`self.K2_GetActorRotation` Terrain)) -1.0)) (`self.GetActorScale3D` Terrain)) "Undefined" "OverrideRootScale" null null))
    (bind _returnvalue_3 (`KismetArrayLibrary.Array_Add` (`self.MirrorObjects`) _returnvalue_2))
    (`TerrainMover.MirrorStates` _returnvalue_2)
    (`KismetSystemLibrary.PrintString` (`KismetStringLibrary.Concat_StrStr` "Spawned new Basewall: " (`KismetStringLibrary.Conv_IntToString` _returnvalue_3) ", at position: " (`KismetStringLibrary.Conv_VectorToString` (`self.K2_GetActorLocation` _returnvalue_2))))
    (else
      (`KismetSystemLibrary.PrintString` "could not find class of parameter terrain mover"))))

(fn `UserConstructionScript`)