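; Health pickup actor that fully restores the player's health when collected.
; Its OnPickup event checks that the collecting actor is a PlayerCharacter, then sets that character's HealthComponent CurrentHealth directly to MaxHealth.
; It prints the restored value on screen in green and destroys itself.
; The overlap event is an empty stub, so this graph does not show what triggers OnPickup.
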(event `self.OnPickup`
  (params (ActorThatPickedUp :type "Actor Object Reference"))
  (if (`KismetMathLibrary.ClassIsChildOf` (`GameplayStatics.GetObjectClass` ActorThatPickedUp) "/Script/AdvGamesProgramming.PlayerCharacter")
    (bind _asplayer_character (cast `PlayerCharacter` ActorThatPickedUp))
    (bind _returnvalue (`self.GetComponentByClass` _asplayer_character "/Script/AdvGamesProgramming.HealthComponent"))
    (bind _output_get (set `HealthComponent.CurrentHealth` (`HealthComponent.MaxHealth` _returnvalue) _returnvalue))
    (`KismetSystemLibrary.PrintString` (`KismetStringLibrary.Conv_DoubleToString` _output_get) true true (struct :`R` 0.170713 :`G` 1.0 :`B` 0.20792 :`A` 1.0))
    (`KismetSystemLibrary.PrintString` "Health Restored To" true true (struct :`R` 0.170713 :`G` 1.0 :`B` 0.20792 :`A` 1.0))
    (`self.K2_DestroyActor`)))

(fn `UserConstructionScript`)