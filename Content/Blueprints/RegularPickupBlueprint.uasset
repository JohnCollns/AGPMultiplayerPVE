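; Stat pickup actor that permanently boosts the player's health or gun stats, then destroys itself.
; BeginPlay calls OnGenerate, then sets the mesh material to match the pickup's Rarity.
; OnPickup requires a PlayerCharacter with a ChildActorComponent and switches on PickupStat.
; It adds to current and max health, or to the child-actor gun's magazine, damage, accuracy or muzzle velocity, with debug prints.
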(event `self.ReceiveBeginPlay`
  (`self.OnGenerate`)
  (switch `EPickupRarity` (`self.Rarity`)
    (:`LEGENDARY`
      (`PrimitiveComponent.SetMaterial` (`self.StaticMesh`) 0 "/Game/Materials/PickupMaterials/LegendaryMaterial.LegendaryMaterial"))
    (:`MASTER`
      (`PrimitiveComponent.SetMaterial` (`self.StaticMesh`) 0 "/Game/Materials/PickupMaterials/MasterMaterial.MasterMaterial"))
    (:`RARE`
      (`PrimitiveComponent.SetMaterial` (`self.StaticMesh`) 0 "/Game/Materials/PickupMaterials/RareMaterial.RareMaterial"))
    (:`COMMON`
      (`PrimitiveComponent.SetMaterial` (`self.StaticMesh`) 0 "/Game/Materials/PickupMaterials/CommonMaterial.CommonMaterial"))))

(event `self.OnPickup`
  (params (ActorThatPickedUp :type "Actor Object Reference"))
  (bind _returnvalue (`self.GetComponentByClass` ActorThatPickedUp "/Script/Engine.ChildActorComponent"))
  (bind _pickupbulletdamage (`self.PickupBulletDamage`))
  (bind _pickuphealth (`self.PickupHealth`))
  (bind _pickupmuzzlevelocity (`self.PickupMuzzleVelocity`))
  (bind _pickupweaponaccuracy (`self.PickupWeaponAccuracy`))
  (bind _pickupmagazinesize (`self.PickupMagazineSize`))
  (if (`KismetMathLibrary.ClassIsChildOf` (`GameplayStatics.GetObjectClass` ActorThatPickedUp) "/Script/AdvGamesProgramming.PlayerCharacter")
    (`/Engine/EditorBlueprintResources/StandardMacros.IsValid` _returnvalue
      (:`Is Valid`
        (switch `EPickupStat` (`self.PickupStat`)
          (:`HEALTH`
            (bind _asplayer_character (cast `PlayerCharacter` ActorThatPickedUp))
            (bind _returnvalue_2 (`self.GetComponentByClass` _asplayer_character "/Script/AdvGamesProgramming.HealthComponent"))
            (set `HealthComponent.CurrentHealth` (+ (`HealthComponent.CurrentHealth` _returnvalue_2) (`self.PickupHealth`)) _returnvalue_2)
            (set `HealthComponent.MaxHealth` (+ (`HealthComponent.MaxHealth` _returnvalue_2) _pickuphealth) _returnvalue_2)
            (`KismetSystemLibrary.PrintString` (`KismetStringLibrary.Conv_DoubleToString` _pickuphealth) true true (struct :`R` 0.983459 :`G` 0.011514 :`B` 1.0 :`A` 1.0))
            (`KismetSystemLibrary.PrintString` "Health Added")
            (`self.K2_DestroyActor`))
          (:`AMMO`
            (bind _asgun_blueprint (cast `/Game/Blueprints/GunBlueprint` (`ChildActorComponent.ChildActor` _returnvalue)))
            (set `/Game/Blueprints/GunBlueprint.MagazineSize` (+ (`/Game/Blueprints/GunBlueprint.MagazineSize` _asgun_blueprint) (`self.PickupMagazineSize`)) _asgun_blueprint)
            (set `/Game/Blueprints/GunBlueprint.RoundsRemainingInMagazine` (+ (`/Game/Blueprints/GunBlueprint.RoundsRemainingInMagazine` _asgun_blueprint) _pickupmagazinesize) _asgun_blueprint)
            (`KismetSystemLibrary.PrintString` (`KismetStringLibrary.Conv_IntToString` _pickupmagazinesize) true true (struct :`R` 0.983459 :`G` 0.011514 :`B` 1.0 :`A` 1.0))
            (`KismetSystemLibrary.PrintString` "Ammo Added" true true (struct :`R` 0.995748 :`B` 1.0 :`A` 1.0))
            (`self.K2_DestroyActor`))
          (:`DAMAGE`
            (bind _asgun_blueprint_2 (cast `/Game/Blueprints/GunBlueprint` (`ChildActorComponent.ChildActor` _returnvalue)))
            (set `/Game/Blueprints/GunBlueprint.BulletDamage` (+ (`/Game/Blueprints/GunBlueprint.BulletDamage` _asgun_blueprint_2) _pickupbulletdamage) _asgun_blueprint_2)
            (`KismetSystemLibrary.PrintString` (`KismetStringLibrary.Conv_DoubleToString` _pickupbulletdamage) true true (struct :`R` 0.983459 :`G` 0.011514 :`B` 1.0 :`A` 1.0))
            (`KismetSystemLibrary.PrintString` "Damage Added" true true (struct :`R` 1.0 :`B` 0.960322 :`A` 1.0))
            (`self.K2_DestroyActor`))
          (:`ACCURACY`
            (bind _asgun_blueprint_3 (cast `/Game/Blueprints/GunBlueprint` (`ChildActorComponent.ChildActor` _returnvalue)))
            (set `/Game/Blueprints/GunBlueprint.WeaponAccuracy` (+ (`/Game/Blueprints/GunBlueprint.WeaponAccuracy` _asgun_blueprint_3) _pickupweaponaccuracy) _asgun_blueprint_3)
            (`KismetSystemLibrary.PrintString` (`KismetStringLibrary.Conv_DoubleToString` _pickupweaponaccuracy) true true (struct :`R` 0.983459 :`G` 0.011514 :`B` 1.0 :`A` 1.0))
            (`KismetSystemLibrary.PrintString` "Accuracy Added" true true (struct :`R` 1.0 :`B` 0.840064 :`A` 1.0))
            (`self.K2_DestroyActor`))
          (:`VELOCITY`
            (bind _asgun_blueprint_4 (cast `/Game/Blueprints/GunBlueprint` (`ChildActorComponent.ChildActor` _returnvalue)))
            (set `/Game/Blueprints/GunBlueprint.MuzzleVelocity` (+ (`/Game/Blueprints/GunBlueprint.MuzzleVelocity` _asgun_blueprint_4) _pickupmuzzlevelocity) _asgun_blueprint_4)
            (`KismetSystemLibrary.PrintString` (`KismetStringLibrary.Conv_DoubleToString` _pickupmuzzlevelocity) true true (struct :`R` 0.983459 :`G` 0.011514 :`B` 1.0 :`A` 1.0))
            (`KismetSystemLibrary.PrintString` "Velocity Added" true true (struct :`R` 1.0 :`G` 0.040479 :`B` 0.965821 :`A` 1.0))
            (`self.K2_DestroyActor`)))))))

(fn `UserConstructionScript`)